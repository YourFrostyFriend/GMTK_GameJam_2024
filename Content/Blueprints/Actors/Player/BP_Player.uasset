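; BP_Player is the 2D platformer player character, driven by flipbook sprites.
; On BeginPlay it finds BP_Aimhand and adds the platforming Enhanced Input mapping context.
; Tick selects idle, run, jump or fall flipbooks from movement, with variants when the aim hand's PickUpSystem holds a prop, and teleports the actor keeping only X and Z, pinning Y.
; The F key runs the RestartLevel console command.
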(event EventBeginPlay
  (Variables|Default|SetplyCanUseItems true)
  (bind _returnvalue (Actor|GetActorOfClass "/Game/Blueprints/Actors/Player/BP_Aimhand.BP_Aimhand_C"))
  (Variables|Default|SetAimhandRef _returnvalue)
  (CallFunction|MapPlyController()))

(event EventTick
  (params (DeltaSeconds :type Float%20%28single-precision%29))
  (bind _returnvalue (Transformation|GetActorLocation))
  (Utilities|FlowControl|Delay 0.0)
  (CallFunction|UpdAnimation())
  (Transformation|SetActorRelativeLocation (Math|Vector|MakeVector (.x _returnvalue) 0.0 (.z _returnvalue)) false true))

(event Input|KeyboardEvents|F
  (params (Key :type Key%20Structure :default "None"))
  (:Pressed
    (Development|ExecuteConsoleCommand "RestartLevel" 0)))

(fn ConstructionScript)

(fn UpdAnimation()
  (bind _sprite (Variables|Default|GetSprite))
  (bind _sprite_2 (Variables|Default|GetSprite))
  (if (AI|Components|NavMovement|IsMovingonGround (Variables|Character|GetCharacterMovement))
    (if (> (Math|Vector|VectorLength (Transformation|GetVelocity)) 0.0)
      (if (Variables|/Game/Blueprints/ActorComponents/Pickup/AC_Pickup.AC_Pickup_C|GetIsHoldingProp (Variables|/Game/Blueprints/Actors/Player/BP_Aimhand.BP_Aimhand_C|GetPick%20Up%20System (Variables|Default|GetAimhandRef)))
        (Sprite|SetFlipbook _sprite_2 "/Game/Assets/Flipbooks/Player_Running_2.Player_Running_2")
        (else
          (Sprite|SetFlipbook _sprite_2 "/Game/Assets/Flipbooks/Character_Run_New.Character_Run_New")))
      (elif (Variables|/Game/Blueprints/ActorComponents/Pickup/AC_Pickup.AC_Pickup_C|GetIsHoldingProp (Variables|/Game/Blueprints/Actors/Player/BP_Aimhand.BP_Aimhand_C|GetPick%20Up%20System (Variables|Default|GetAimhandRef)))
        (Sprite|SetFlipbook _sprite_2 "/Game/Assets/Flipbooks/Player_Idle_2.Player_Idle_2")
        (else
          (Sprite|SetFlipbook _sprite_2 "/Game/Assets/Sprites/Player/Player_Idle.Player_Idle"))))
    (elif (< (.z (Transformation|GetVelocity)) -1e+02)
      (if (Variables|/Game/Blueprints/ActorComponents/Pickup/AC_Pickup.AC_Pickup_C|GetIsHoldingProp (Variables|/Game/Blueprints/Actors/Player/BP_Aimhand.BP_Aimhand_C|GetPick%20Up%20System (Variables|Default|GetAimhandRef)))
        (Sprite|SetFlipbook _sprite "/Game/Assets/Flipbooks/Player_Falling_2.Player_Falling_2")
        (else
          (Sprite|SetFlipbook _sprite "/Game/Assets/Flipbooks/Player_Falling.Player_Falling")))
      (elif (Variables|/Game/Blueprints/ActorComponents/Pickup/AC_Pickup.AC_Pickup_C|GetIsHoldingProp (Variables|/Game/Blueprints/Actors/Player/BP_Aimhand.BP_Aimhand_C|GetPick%20Up%20System (Variables|Default|GetAimhandRef)))
        (Sprite|SetFlipbook _sprite "/Game/Assets/Flipbooks/Player_Jumping_2.Player_Jumping_2")
        (else
          (Sprite|SetFlipbook _sprite "/Game/Assets/Flipbooks/Player_Jump.Player_Jump"))))))

(fn MapPlyController()
  (bind _asplayer_controller (Utilities|Casting|CastToPlayerController (Pawn|GetController)))
  (Input|AddMappingContext (PlayerController|LocalPlayerSubsystems|GetEnhancedInputLocalPlayerSubsystem _asplayer_controller) "/Game/Data/Input/IMC_Platforming.IMC_Platforming" 0 "(bIgnoreAllPressedKeysUntilRelease=True,bForceImmediately=False,bNotifyUserSettings=False)"))