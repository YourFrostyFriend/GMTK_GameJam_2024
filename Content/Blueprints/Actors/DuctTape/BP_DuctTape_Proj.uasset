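; BP_DuctTape_Proj is a duct tape projectile that tapes objects it hits.
; On actor hit, ignoring the BP_Player and BP_Aimhand references, it calls EventTapeHit on a BP_Object.
; Any other hit instead refunds one unit to DuctTapeAmount in the game instance.
; After either outcome it prints the current tape count and destroys itself.
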(event Custom|OnActorHit_Event
  (params (SelfActor :type Actor%20Object%20Reference) (OtherActor :type Actor%20Object%20Reference) (NormalImpulse :type Vector) (Hit :type Hit%20Result%20Structure%20%28by%20ref%29))
  (if (not (or (== OtherActor "/Game/Blueprints/Actors/Player/BP_Player.BP_Player") (== OtherActor "/Game/Blueprints/Actors/Player/BP_Aimhand.BP_Aimhand")))
    (bind _asbp_object (Utilities|Casting|CastToBP_Object OtherActor)
      (:then
        (Default|EventTapeHit _asbp_object))
      (:CastFailed
        (Variables|/Game/Blueprints/Utility/Transitions/BP_Game_Instance.BP_Game_Instance_C|SetDuctTapeAmount (stale EventBeginPlay _asbp_game_instance) (+ (Variables|/Game/Blueprints/Utility/Transitions/BP_Game_Instance.BP_Game_Instance_C|GetDuctTapeAmount (stale EventBeginPlay _asbp_game_instance)) 1))))
    (Development|PrintText (Utilities|Text|ToText(Integer) (Variables|/Game/Blueprints/Utility/Transitions/BP_Game_Instance.BP_Game_Instance_C|GetDuctTapeAmount (stale EventBeginPlay _asbp_game_instance))))
    (Actor|DestroyActor)))

(event EventBeginPlay
  (EventDispatchers|BindEventtoOnActorHit (delegate Custom|OnActorHit_Event))
  (bind _asbp_game_instance (Utilities|Casting|CastToBP_Game_Instance (Game|GetGameInstance))))

(event Collision|EventActorBeginOverlap
  (params (OtherActor :type Actor%20Object%20Reference)))

(event EventTick
  (params (DeltaSeconds :type Float%20%28single-precision%29)))

(fn ConstructionScript)