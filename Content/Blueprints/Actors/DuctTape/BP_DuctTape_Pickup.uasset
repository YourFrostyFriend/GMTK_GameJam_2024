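; Pickup actor that grants duct tape to the player when touched.
; On BeginPlay it caches the game instance as BP_Game_Instance.
; When BP_Player overlaps its Box, it adds GiveAmount to the game instance's DuctTapeAmount, then destroys itself.
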(event OnComponentBeginOverlap(Box)
  (params (OverlappedComponent :type Primitive%20Component%20Object%20Reference) (OtherActor :type Actor%20Object%20Reference) (OtherComp :type Primitive%20Component%20Object%20Reference) (OtherBodyIndex :type Integer) (bFromSweep :type Boolean) (SweepResult :type Hit%20Result%20Structure%20%28by%20ref%29))
  (bind _gameinstanceref (Variables|Default|GetGameInstanceRef))
  (Utilities|Casting|CastToBP_Player OtherActor)
  (Variables|/Game/Blueprints/Utility/Transitions/BP_Game_Instance.BP_Game_Instance_C|SetDuctTapeAmount _gameinstanceref (+ (Variables|/Game/Blueprints/Utility/Transitions/BP_Game_Instance.BP_Game_Instance_C|GetDuctTapeAmount _gameinstanceref) (Variables|Default|GetGiveAmount)))
  (Actor|DestroyActor))

(event EventBeginPlay
  (bind _asbp_game_instance (Utilities|Casting|CastToBP_Game_Instance (Game|GetGameInstance)))
  (Variables|Default|SetGameInstanceRef _asbp_game_instance))

(event EventTick
  (params (DeltaSeconds :type Float%20%28single-precision%29)))

(fn ConstructionScript)