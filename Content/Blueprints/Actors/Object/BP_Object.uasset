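; Sprite-based physics object that the player's enlarge and shrink rays resize and duct tape freezes in place.
; ScaleGunHit steps a capped scale counter, and timelines lerp the sprite's X and Z scale.
; TapeHit makes the sprite static with an overlay; a valid resize unfreezes it and spawns a tape pickup.
; Explodable objects at maximum size burst after a delay, launching a nearby player via sphere trace.
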(event Custom|Event%20Scale%20Gun%20Hit
  (params (ScaleHitData :type STRCT%20Scale%20Gun%20Hit%20Data%20Structure))
  (bind _sprite (Variables|Default|GetSprite))
  (bind _sprite_2 (Variables|Default|GetSprite))
  (bind _sprite_3 (Variables|Default|GetSprite))
  (bind _returnvalue (Transformation|GetWorldScale _sprite_2))
  (bind _returnvalue_2 (Transformation|GetWorldScale _sprite))
  (if (not (Variables|Default|GetisShaping))
    (Utilities|FlowControl|Sequence
      (:then_0
        ;[1 1 1] For Enlarge Ray
        (if (Utilities|IsValid (.instigator ScaleHitData))
          (if (and (< (Variables|Default|GetcurScaleNum) (Variables|Default|GetlimitScaleNum)) (Utilities|Enum|Equal(Enum) "NewEnumerator0" (.hittype ScaleHitData)))
            (CallFunction|TapeFreezeSelf() false)
            (bind _return_multiplier (CallFunction|AddScaleMultiplier() (.scalemultiplier ScaleHitData)))
            (Variables|Default|SetcurScaleNum (+ (Variables|Default|GetcurScaleNum) 1.0))
            (Variables|Default|SetisShaping true)
            (bind _alphavalue (Timeline|Timeline_0 PlayFromStart)
              (:Update
                (Transformation|SetRelativeScale3D (Variables|Default|GetSprite) (Math|Vector|MakeVector (Math|Float|Lerp (.x _returnvalue_2) _return_multiplier _alphavalue) (.y _returnvalue_2) (Math|Float|Lerp (.x _returnvalue_2) _return_multiplier _alphavalue))))
              (:Finished
                (Variables|Default|SetisShaping false)
                (if (and (Variables|Default|GetCanExplode) (>= (Variables|Default|GetcurScaleNum) (Variables|Default|GetlimitScaleNum)))
                  (Class|PrimitiveComponent|SetAngularDamping _sprite_3 1e+02)
                  (Class|PrimitiveComponent|SetPhysMaterialOverride _sprite_3)
                  (Utilities|FlowControl|Delay 2.0)
                  (CallFunction|AirExplode())
                  (Actor|DestroyActor)))))))
      (:then_1
        ;[1 1 1] For Shrink Ray
        (if (Utilities|IsValid (.instigator ScaleHitData))
          (if (and (> (Variables|Default|GetcurScaleNum) (- 0.0 (Variables|Default|GetlimitScaleNum))) (Utilities|Enum|Equal(Enum) "NewEnumerator1" (.hittype ScaleHitData)))
            (CallFunction|TapeFreezeSelf() false)
            (bind _return_multiplier_2 (CallFunction|AddScaleMultiplier() (.scalemultiplier ScaleHitData)))
            (Variables|Default|SetcurScaleNum (- (Variables|Default|GetcurScaleNum) 1.0))
            (Variables|Default|SetisShaping true)
            (bind _alphavalue_2 (Timeline|Timeline PlayFromStart)
              (:Update
                (Transformation|SetRelativeScale3D (Variables|Default|GetSprite) (Math|Vector|MakeVector (Math|Float|Lerp (.x _returnvalue) _return_multiplier_2 _alphavalue_2) (.y _returnvalue) (Math|Float|Lerp (.x _returnvalue) _return_multiplier_2 _alphavalue_2))))
              (:Finished
                (Variables|Default|SetisShaping false)))))))))

(event Custom|Event%20Tape%20Hit
  (if (not (Variables|Default|GetisTaped))
    (CallFunction|TapeFreezeSelf() true)))

(event EventBeginPlay
  (Variables|Default|SetcurScaleMultiplier (.x (Variables|/Script/Engine.SceneComponent|GetRelativeScale3D (Variables|Default|GetSprite))))
  (Variables|Default|SetlimitScaleNum 3.0))

(event Collision|EventActorBeginOverlap
  (params (OtherActor :type Actor%20Object%20Reference)))

(event EventTick
  (params (DeltaSeconds :type Float%20%28single-precision%29)))

(fn ConstructionScript)

(fn AddScaleMultiplier()
  (params (Multiplier :type Float%20%28double-precision%29))
  (if (not (<= (+ (- Multiplier 1.0) (Variables|Default|GetcurScaleMultiplier)) 0.0))
    (bind _output_get (Variables|Default|SetcurScaleMultiplier (+ (- Multiplier 1.0) (Variables|Default|GetcurScaleMultiplier))))
    (return _output_get)))

(fn SettoInactive()
  (params (Inactive :type Boolean))
  (if Inactive
    (Rendering|SetVisibility (Variables|Default|GetSprite) false false)
    (Physics|SetSimulatePhysics (Variables|Default|GetSprite) false)
    (Collision|SetCollisionEnabled (Variables|Default|GetSprite) "NoCollision")
    (else
      (Rendering|SetVisibility (Variables|Default|GetSprite) true false)
      (Physics|SetSimulatePhysics (Variables|Default|GetSprite) true)
      (Collision|SetCollisionEnabled (Variables|Default|GetSprite) "QueryAndPhysics"))))

(fn TapeFreezeSelf()
  (params (IsFrozen :type Boolean))
  (bind _returnvalue (Transformation|GetActorTransform))
  (bind _self self)
  (bind _self_2 self)
  (bind _returnvalue_2 (Transformation|GetActorTransform _self_2))
  (bind _returnvalue_3 (Transformation|GetActorTransform _self))
  (if IsFrozen
    (Variables|Default|SetisTaped true)
    (Transformation|Teleport _self (.location _returnvalue_3) (.rotation _returnvalue_3))
    (Transformation|SetMobility (Variables|Default|GetSprite) "Static")
    (Rendering|SetVisibility (Variables|Default|GetTapeOverlay) true false)
    (Audio|PlaySound2D "/Game/Assets/Audio/S_ApplyTape.S_ApplyTape" 1.0 1.0 0.0 0 0)
    (return)
    (elif (== (Variables|Default|GetisTaped) true)
      (Variables|Default|SetisTaped false)
      (Transformation|Teleport _self_2 (.location _returnvalue_2) (.rotation _returnvalue_2))
      (Transformation|SetMobility (Variables|Default|GetSprite) "Movable")
      (Game|SpawnActorfromClass "/Game/Blueprints/Actors/DuctTape/BP_DuctTape_Pickup.BP_DuctTape_Pickup_C" (Math|Transform|MakeTransform (Math|Vector|MakeVector (.x (.location _returnvalue)) (.y (.location _returnvalue)) (+ (.z (.location _returnvalue)) 4e+01)) "0, 0, 0" "1.000000,1.000000,1.000000") "AdjustIfPossibleButAlwaysSpawn" "MultiplyWithRoot" 0 0)
      (Rendering|SetVisibility (Variables|Default|GetTapeOverlay) false false)
      (Audio|PlaySound2D "/Game/Assets/Audio/S_ApplyTape.S_ApplyTape" 1.0 1.0 0.0 0 0)
      (return))))

(fn AirExplode()
  (bind _returnvalue (Transformation|GetActorLocation))
  (bind _outhit (Collision|SphereTraceForObjects _returnvalue _returnvalue 6e+02 (Utilities|Array|MakeArray "ObjectTypeQuery3") false 0 "None"))
  (bind _asbp_player (Utilities|Casting|CastToBP_Player (.hitactor _outhit))
    (:then
      (Character|LaunchCharacter _asbp_player (* (Math|Vector|Normalize (- (.impactpoint _outhit) (Transformation|GetActorLocation))) 1.7e+03) true true)
      (Development|PrintText (Utilities|Text|ToText(String) (- (.impactpoint _outhit) (Transformation|GetActorLocation)))))
    (:CastFailed
      (return))))