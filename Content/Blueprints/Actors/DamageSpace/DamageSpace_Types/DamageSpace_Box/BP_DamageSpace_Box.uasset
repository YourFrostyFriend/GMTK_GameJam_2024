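; BP_DamageSpace_Box is a box-type damage space actor that updates the target list of its stored damage info on actor overlap.
; On overlap it scans the targets, setting ActorExists when the other actor is already listed and is not the source.
; When that flag is true it appends the actor, so only already-listed actors trigger an add; the flag is never reset here.
; BeginPlay and construction defer to the parent.
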(event EventBeginPlay
  (|CallParentFunction))

(event Collision|EventActorBeginOverlap
  (params (OtherActor :type Actor%20Object%20Reference))
  ;[1 0.9169 0.1874] Set DamageInfo's Target to all objects that is in DamageSpace
  (for _array_element (.target (Variables|Default|GetStoredDamageInfo))
    (if (and (!= OtherActor (.source (Variables|Default|GetStoredDamageInfo))) (== OtherActor _array_element))
      (Variables|Default|SetActorExists true)))
  (if (Variables|Default|GetActorExists)
    (Utilities|Array|Add (.target (Variables|Default|GetStoredDamageInfo)) OtherActor)
    (Variables|Default|SetStoredDamageInfo (Utilities|Struct|MakeSTRUCT_DamageInfo (.source (Variables|Default|GetStoredDamageInfo)) (.target (Variables|Default|GetStoredDamageInfo)) (.amount (Variables|Default|GetStoredDamageInfo)) "NewEnumerator0"))))

(fn ConstructionScript
  (|CallParentFunction))