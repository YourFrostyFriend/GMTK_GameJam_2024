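; Pickup actor that grants the player the Scalegun.
; On BeginPlay it caches the game instance and finds the BP_Aimhand actor in the level.
; When BP_Player overlaps its box, it sets the has-gun flag on the game instance, changes the crosshair cursor through the Aimhand's UI reference, and destroys itself.
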(event OnComponentBeginOverlap(Box)
  (params (OverlappedComponent :type Primitive%20Component%20Object%20Reference) (OtherActor :type Actor%20Object%20Reference) (OtherComp :type Primitive%20Component%20Object%20Reference) (OtherBodyIndex :type Integer) (bFromSweep :type Boolean) (SweepResult :type Hit%20Result%20Structure%20%28by%20ref%29))
  (Utilities|Casting|CastToBP_Player OtherActor)
  (Variables|/Game/Blueprints/Utility/Transitions/BP_Game_Instance.BP_Game_Instance_C|SetPlyHasGun (Variables|Default|GetGameInstanceRef) true)
  (Default|ChangeCursor (Variables|/Game/Blueprints/Actors/Player/BP_Aimhand.BP_Aimhand_C|GetCrosshairUIRef (Variables|Default|GetAimhandRef)) "NewEnumerator0")
  (Actor|DestroyActor))

(event EventBeginPlay
  (bind _asbp_game_instance (Utilities|Casting|CastToBP_Game_Instance (Game|GetGameInstance)))
  (Variables|Default|SetGameInstanceRef _asbp_game_instance)
  (bind _returnvalue (Actor|GetActorOfClass "/Game/Blueprints/Actors/Player/BP_Aimhand.BP_Aimhand_C"))
  (Variables|Default|SetAimhandRef _returnvalue))

(event EventTick
  (params (DeltaSeconds :type Float%20%28single-precision%29)))

(fn ConstructionScript)