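; BP_Camera is a stage camera for a side-view game that follows the player on X and Z within a confines box.
; The construction script sizes that box from stage width and height in screen multiples and places the player trigger box.
; Overlapping the trigger, or starting inside it, makes this the player's current camera and view target.
; Each tick interpolates toward the player, then clamps to bounds inset by half a screen.
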(event OnComponentBeginOverlap(PlayerTriggerBox)
  (params (OverlappedComponent :type Primitive%20Component%20Object%20Reference) (OtherActor :type Actor%20Object%20Reference) (OtherComp :type Primitive%20Component%20Object%20Reference) (OtherBodyIndex :type Integer) (bFromSweep :type Boolean) (SweepResult :type Hit%20Result%20Structure%20%28by%20ref%29))
  (bind _asbp_player (Utilities|Casting|CastToBP_Player OtherActor))
  (Variables|/Game/Blueprints/Actors/Player/BP_Player.BP_Player_C|SetCurrent%20Camera _asbp_player self)
  (Game|Player|SetViewTargetwithBlend (Game|GetPlayerController 0) self 0.0 "VTBlend_Linear" 0.0 false))

(event EventBeginPlay
  (Utilities|GetConfinesBoxBounds
    (:Out
      (Utilities|FlowControl|Delay 0.0)
      (bind _asbp_player (Utilities|Casting|CastToBP_Player (Game|Player|GetPlayerPawn 0)))
      (for _array_element (Class|Actor|GetOverlappingComponents _asbp_player)
        (if (== _array_element (Variables|Default|GetPlayer%20Trigger%20Box))
          (Variables|/Game/Blueprints/Actors/Player/BP_Player.BP_Player_C|SetCurrent%20Camera _asbp_player self)
          (Game|Player|SetViewTargetwithBlend (Game|GetPlayerController 0) self 0.0 "VTBlend_Linear" 0.0 false))))))

(event EventTick
  (params (DeltaSeconds :type Float%20%28single-precision%29))
  (Variables|Default|SetDelta%20Time DeltaSeconds)
  (Utilities|CameraFollowPlayerX
    (:Out
      (Utilities|CameraFollowPlayerZ
        (:Out
          (Utilities|LerpWithinConfines
            (:Out
              (Utilities|SetCameraPosition))))))))

(fn ConstructionScript
  (Transformation|SetRelativeTransform (Variables|Default|GetPlayer%20Trigger%20Box) (Variables|Triggers|GetPlayer%20Trigger%20Transform) false false)
  (Components|Box|SetBoxExtent (Variables|Default|GetPlayer%20Trigger%20Box) (Variables|Triggers|GetPlayer%20Trigger%20Extent) true)
  (Components|Box|SetBoxExtent (Variables|Default|GetCamera%20Confines%20Box) (Math|Vector|MakeVector (Math|Conversions|ToFloat(Integer) (* (* (Variables|StageSize|GetStage%20Width) 16) 35)) 1e+01 (Math|Conversions|ToFloat(Integer) (* (* (Variables|StageSize|GetStage%20Height) 16) 22))) true))

(fn ZoomOut
  (Transformation|SetWorldLocation (Variables|Default|GetCamera) "0, 0, 0" false false))