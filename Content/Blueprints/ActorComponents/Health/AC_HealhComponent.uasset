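; Actor component that holds a health value for its owning actor, with damage handling left unfinished.
; On BeginPlay it fills Health to MaxHealth and binds to the owner's begin-overlap event, whose handler is empty.
; An unconnected damage branch checks FindOwnerInArray, subtracts zero and prints remaining health.
; That helper casts the owner's Find index straight to a bool, so it does not reliably test membership.
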(event Custom|OnActorBeginOverlap_Event
  (params (OverlappedActor :type Actor%20Object%20Reference) (OtherActor :type Actor%20Object%20Reference)))

(event EventBeginPlay
  ;[1 0.9269 0.1705] Set Entity Health to Max Health
  (Variables|Default|SetHealth (Variables|Default|GetMaxHealth))
  (EventDispatchers|AssignOnActorBeginOverlap (Components|GetOwner) (delegate Custom|OnActorBeginOverlap_Event)))

(fn FindOwnerinArray()
  (params (Array :type Array%20of%20Actor%20Object%20References))
  (if (Math|Conversions|ToBoolean(Integer) (Utilities|Array|FindItem Array (Components|GetOwner)))
    (LocalVariables|SetOutputBool true))
  (return (LocalVariables|GetOutputBool)))