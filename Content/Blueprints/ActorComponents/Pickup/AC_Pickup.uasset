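; Actor component that lets the player pick up and throw sprite-based BP_Object props with the interact input.
; A trace toward AC_Scalegun's mouse location grabs nearby, untaped, small-enough props, deactivating them and mirroring their sprite on the player's HeldDisplay.
; While a prop is held, item use is disabled.
; Interacting again teleports it above the player, reactivates it and launches it toward the cursor with a minimum upward bias.
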(event Input|EnhancedActionEvents|EnhancedInputActionIA_Interact
  (params (ActionValue :type Boolean) (ElapsedSeconds :type Float%20%28double-precision%29) (TriggeredSeconds :type Float%20%28double-precision%29) (InputAction :type Input%20Action%20Object%20Reference :default "/Game/Data/Input/InputActions/IA_Interact.IA_Interact"))
  (bind _playerref (Variables|Default|GetPlayerRef))
  (bind _playerref_2 (Variables|Default|GetPlayerRef))
  (bind _scaleguncomponent (Variables|Default|GetScalegunComponent))
  (bind _playerref_3 (Variables|Default|GetPlayerRef))
  (bind _playerref_4 (Variables|Default|GetPlayerRef))
  (bind _returnvalue (Transformation|GetActorLocation _playerref_2))
  (bind _rootcomponent (Variables|/Script/Engine.Actor|GetRootComponent _playerref_3))
  (bind _curmouselocation (Variables|/Game/Blueprints/ActorComponents/Items/AC_Scalegun.AC_Scalegun_C|GetcurMouseLocation _scaleguncomponent))
  (bind _helddisplay (Variables|/Game/Blueprints/Actors/Player/BP_Player.BP_Player_C|GetHeldDisplay _playerref_4))
  (bind _returnvalue_2 (Transformation|GetWorldLocation _rootcomponent))
  (bind _returnvalue_3 (- _curmouselocation _returnvalue_2))
  (bind (_x _y _z) (Math|Vector|BreakVector _returnvalue_3))
  (:Started
    (if (Variables|Default|GetIsHoldingProp)
      (Variables|Default|SetIsHoldingProp false)
      (Transformation|Teleport (Variables|Default|GetcurHeldItem) (Math|Vector|MakeVector (.x _returnvalue) (.y (Transformation|GetWorldLocation (Variables|/Script/Engine.Actor|GetRootComponent (Variables|Default|GetcurHeldItem)))) (+ (.z _returnvalue) 7e+01)) "0, 0, 0")
      (Default|SettoInactive() (Variables|Default|GetcurHeldItem) false)
      (Rendering|Components|Sprite|SetSprite (Variables|/Game/Blueprints/Actors/Player/BP_Player.BP_Player_C|GetHeldDisplay _playerref) 0)
      (Physics|AddImpulse (Variables|/Game/Blueprints/Actors/Object/BP_Object.BP_Object_C|GetSprite (Variables|Default|GetcurHeldItem)) (* (Math|Vector|Normalize (Math|Vector|MakeVector _x _y (Math|Float|Clamp(Float) _z 0.5 999999.0))) 6e+02) "None" true)
      (Variables|Default|SetcurHeldItem (Variables|Default|GetEmptyReference))
      (Variables|/Game/Blueprints/Actors/Player/BP_Player.BP_Player_C|SetplyCanUseItems _playerref true)
      (Audio|PlaySound2D "/Game/Assets/Audio/S_Throwing.S_Throwing" 1.0 1.0 0.0 0 0)
      (else
        (bind _outhit (Collision|LineTraceForObjects (Transformation|GetActorLocation _playerref_4) (Variables|/Game/Blueprints/ActorComponents/Items/AC_Scalegun.AC_Scalegun_C|GetcurMouseLocation (Variables|Default|GetScalegunComponent)) (Utilities|Array|MakeArray "ObjectTypeQuery4") false 0 "None"))
        (if (<= (.distance _outhit) 1e+02)
          (bind _asbp_object (Utilities|Casting|CastToBP_Object (.hitactor _outhit)))
          (if (not (Variables|/Game/Blueprints/Actors/Object/BP_Object.BP_Object_C|GetisTaped _asbp_object))
            (if (< (.SphereRadius (Collision|GetComponentBounds (Variables|/Game/Blueprints/Actors/Object/BP_Object.BP_Object_C|GetSprite _asbp_object))) 78.0)
              (Variables|/Game/Blueprints/Actors/Player/BP_Player.BP_Player_C|SetplyCanUseItems (Variables|Default|GetPlayerRef) false)
              (Variables|Default|SetcurHeldItem _asbp_object)
              (Variables|Default|SetIsHoldingProp true)
              (Default|SettoInactive() (Variables|Default|GetcurHeldItem) true)
              (Rendering|Components|Sprite|SetSprite _helddisplay (Sprite|GetSprite (Variables|/Game/Blueprints/Actors/Object/BP_Object.BP_Object_C|GetSprite (Variables|Default|GetcurHeldItem))))
              (Transformation|SetRelativeScale3D _helddisplay (Transformation|GetWorldScale (Variables|/Game/Blueprints/Actors/Object/BP_Object.BP_Object_C|GetSprite (Variables|Default|GetcurHeldItem)))))))))))

(event EventBeginPlay
  (Variables|Default|SetScalegunComponent (Actor|GetComponentbyClass (Components|GetOwner) "/Game/Blueprints/ActorComponents/Items/AC_Scalegun.AC_Scalegun_C"))
  (bind _returnvalue (Actor|GetActorOfClass "/Game/Blueprints/Actors/Player/BP_Player.BP_Player_C"))
  (Variables|Default|SetPlayerRef _returnvalue))

(fn FindAngleBetweenVectors()
  (params (A :type Vector) (B :type Vector))
  (bind _returnvalue (Math|Vector|Normalize B))
  (bind _returnvalue_2 (Math|Vector|Normalize A))
  (bind _returnvalue_3 (Math|Vector|DotProduct _returnvalue_2 _returnvalue))
  (bind _returnvalue_4 (Class|KismetMathLibrary|DegAcos _returnvalue_3))
  (Development|PrintText (Utilities|Text|ToText(Float) _returnvalue_4 "HalfToEven"))
  (return _returnvalue_4))