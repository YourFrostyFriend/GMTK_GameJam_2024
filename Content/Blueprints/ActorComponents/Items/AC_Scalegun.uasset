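; Scale gun component for the aim hand that grows or shrinks BP_Objects with left and right click.
; Each tick it rotates its owner toward the cursor hit point, locked to the owner's Y for aiming in the XZ plane.
; When the player can use items, a click line-traces physics bodies toward that point and passes scale hit data to the hit BP_Object.
; Firing also prints debug text and draws a debug line.
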(event Input|EnhancedActionEvents|EnhancedInputActionIA_Left_Click
  (params (ActionValue :type Boolean) (ElapsedSeconds :type Float%20%28double-precision%29) (TriggeredSeconds :type Float%20%28double-precision%29) (InputAction :type Input%20Action%20Object%20Reference :default "/Game/Data/Input/InputActions/IA_Left_Click.IA_Left_Click"))
  (:Started
    (bind _bool (CallFunction|CanPlyUseItem()))
    (if _bool
      (Development|PrintText "Fire")
      (CallFunction|FireBigRay() (Variables|Default|GetcurMouseLocation) 1.5)
      (Rendering|Debug|DrawDebugLine (Math|Vector|MakeVector 0.0 0.0 0.0) (Math|Vector|MakeVector 0.0 0.0 0.0) "(R=1.000000,G=0.000000,B=0.000000,A=1.000000)" 0.0 5.0))))

(event Input|EnhancedActionEvents|EnhancedInputActionIA_Right_Click
  (params (ActionValue :type Boolean) (ElapsedSeconds :type Float%20%28double-precision%29) (TriggeredSeconds :type Float%20%28double-precision%29) (InputAction :type Input%20Action%20Object%20Reference :default "/Game/Data/Input/InputActions/IA_Right_Click.IA_Right_Click"))
  (:Started
    (bind _bool (CallFunction|CanPlyUseItem()))
    (if _bool
      (Development|PrintText "Fire")
      (CallFunction|FireSmallRay() (Variables|Default|GetcurMouseLocation) 0.5)
      (Rendering|Debug|DrawDebugLine (Math|Vector|MakeVector 0.0 0.0 0.0) (Math|Vector|MakeVector 0.0 0.0 0.0) "(R=1.000000,G=0.000000,B=0.000000,A=1.000000)" 0.0 5.0))))

(event EventBeginPlay
  (Input|EnableInput (Components|GetOwner) (Game|GetPlayerController 0)))

(event EventTick
  (params (DeltaSeconds :type Float%20%28single-precision%29))
  (CallFunction|MouseAimTick()))

(fn MouseAimTick()
  (bind _returnvalue (Game|GetPlayerController 0))
  (bind _returnvalue_2 (Components|GetOwner))
  (bind _returnvalue_3 (Transformation|GetActorLocation _returnvalue_2))
  (bind _hitresult (Game|Player|GetHitResultUnderCursorbyChannel _returnvalue "TraceTypeQuery1" true))
  (Transformation|SetActorRotation _returnvalue_2 (Math|Rotator|FindLookatRotation (Math|Vector|MakeVector (.x _returnvalue_3) (.y _returnvalue_3) (.z _returnvalue_3)) (Math|Vector|MakeVector (.x (.location _hitresult)) (.y _returnvalue_3) (.z (.location _hitresult)))))
  (Variables|Default|SetcurMouseLocation (Math|Vector|MakeVector (.x (.location _hitresult)) (.y _returnvalue_3) (.z (.location _hitresult)))))

(fn FireBigRay()
  (params (TargetLocation :type Vector) (ScaleMultiplier :type Float%20%28double-precision%29))
  (bind _returnvalue (Components|GetOwner))
  (bind _returnvalue_2 (Transformation|GetActorLocation _returnvalue))
  (LocalVariables|SetnewScaleHitData (Utilities|Struct|MakeSTRCT_ScaleGunHitData (Components|GetOwner) "NewEnumerator0" ScaleMultiplier))
  (bind _outhit (Collision|LineTraceForObjects (Math|Vector|MakeVector (.x _returnvalue_2) (.y _returnvalue_2) (.z _returnvalue_2)) (Math|Vector|MakeVector (.x TargetLocation) (.y _returnvalue_2) (.z TargetLocation)) (Utilities|Array|MakeArray "ObjectTypeQuery4") false 0 "None"))
  (bind _asbp_object (Utilities|Casting|CastToBP_Object (.hitactor _outhit)))
  (Default|EventScaleGunHit _asbp_object (LocalVariables|GetnewScaleHitData)))

(fn FireSmallRay()
  (params (TargetLocation :type Vector) (ScaleMultiplier :type Float%20%28double-precision%29))
  (bind _returnvalue (Components|GetOwner))
  (bind _returnvalue_2 (Transformation|GetActorLocation _returnvalue))
  (LocalVariables|SetnewScaleHitData (Utilities|Struct|MakeSTRCT_ScaleGunHitData (Components|GetOwner) "NewEnumerator1" ScaleMultiplier))
  (bind _outhit (Collision|LineTraceForObjects (Math|Vector|MakeVector (.x _returnvalue_2) (.y _returnvalue_2) (.z _returnvalue_2)) (Math|Vector|MakeVector (.x TargetLocation) (.y _returnvalue_2) (.z TargetLocation)) (Utilities|Array|MakeArray "ObjectTypeQuery4") false 0 "None"))
  (bind _asbp_object (Utilities|Casting|CastToBP_Object (.hitactor _outhit)))
  (Default|EventScaleGunHit _asbp_object (LocalVariables|GetnewScaleHitData)))

(fn MapPlyController()
  (bind _asplayer_controller (Utilities|Casting|CastToPlayerController (Pawn|GetController (Game|Player|GetPlayerPawn 0))))
  (Input|AddMappingContext (PlayerController|LocalPlayerSubsystems|GetEnhancedInputLocalPlayerSubsystem _asplayer_controller) "/Game/Data/Input/IMC_Platforming.IMC_Platforming" 0 "(bIgnoreAllPressedKeysUntilRelease=True,bForceImmediately=False,bNotifyUserSettings=False)"))

(fn CanPlyUseItem()
  (bind _asbp_aimhand (Utilities|Casting|CastToBP_Aimhand (Components|GetOwner)))
  (return (Variables|/Game/Blueprints/Actors/Player/BP_Player.BP_Player_C|GetplyCanUseItems (Variables|/Game/Blueprints/Actors/Player/BP_Aimhand.BP_Aimhand_C|GetPlayerRef _asbp_aimhand))))