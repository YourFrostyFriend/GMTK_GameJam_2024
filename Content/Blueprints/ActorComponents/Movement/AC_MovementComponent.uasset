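; Actor component that drives side-scrolling movement and jumping when its owner is BP_Player, staying inactive on other owners.
; BeginPlay caches the character movement component and default values; move input applies speed, moves along world X and snaps controller yaw to face the travel direction.
; Jump uses LaunchCharacter with coyote time, a tick-counted, frame-rate-dependent grace window that resets on the ground and allows one jump.
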(event Input|EnhancedActionEvents|EnhancedInputActionIA_Jump
  (params (ActionValue :type Boolean) (ElapsedSeconds :type Float%20%28double-precision%29) (TriggeredSeconds :type Float%20%28double-precision%29) (InputAction :type Input%20Action%20Object%20Reference :default "/Game/Data/Input/InputActions/IA_Jump.IA_Jump"))
  (:Started
    (if (== (Variables|Default|GetIsPlayer) true)
      (if (and (not (Variables|Default|GetPHasJumped)) (> (Variables|Default|GetPCoyoteTime) 0.0))
        (Character|LaunchCharacter (Class|CharacterMovementComponent|GetCharacterOwner (Variables|Default|GetPlayerMoveCompRef)) (Math|Vector|MakeVector 0.0 0.0 (Variables|Default|GetJumpPower)) false true)
        (Variables|Default|SetPHasJumped true)))))

(event Input|EnhancedActionEvents|EnhancedInputActionIA_Move
  (params (ActionValue :type Float%20%28double-precision%29) (ElapsedSeconds :type Float%20%28double-precision%29) (TriggeredSeconds :type Float%20%28double-precision%29) (InputAction :type Input%20Action%20Object%20Reference :default "/Game/Data/Input/InputActions/IA_Move.IA_Move"))
  (if (== (Variables|Default|GetIsPlayer) true)
    (Variables|/Script/Engine.CharacterMovementComponent|SetMaxWalkSpeed (Variables|Default|GetPlayerMoveCompRef) (Variables|Default|GetSpeed))
    (Pawn|Input|AddMovementInput (Variables|/Script/Engine.Actor|GetInstigator (Components|GetOwner)) "1.000000,0.000000,0.000000" ActionValue false)
    (Pawn|SetControlRotation (Pawn|GetController (Variables|/Script/Engine.Actor|GetInstigator (Components|GetOwner))) (select (> ActionValue 0.0) (Math|Rotator|MakeRotator 0.0 0.0 0.0) (Math|Rotator|MakeRotator 0.0 0.0 1.8e+02)))))

(event EventBeginPlay
  (Utilities|FlowControl|Sequence
    (:then_0
      (CallFunction|SpeedComponentBeginTickPlayer()))))

(event EventTick
  (params (DeltaSeconds :type Float%20%28single-precision%29))
  (CallFunction|MoveCompTickPlayer()))

(fn SpeedComponentBeginTickPlayer()
  (bind _asbp_player (Utilities|Casting|CastToBP_Player (Components|GetOwner))
    (:then
      (Variables|Default|SetPlayerMoveCompRef (Variables|/Script/Engine.Character|GetCharacterMovement _asbp_player))
      (Variables|Default|SetSpeed (Variables|Default|GetDefaultSpeed))
      (Variables|Default|SetJumpPower (Variables|Default|GetDefaultJumpPower))
      (Variables|Default|SetPCoyoteTime (Variables|Default|GetPDefaultCoyoteTime))
      (Variables|Default|SetIsPlayer true))
    (:CastFailed
      (Variables|Default|SetIsPlayer false))))

(fn MoveCompTickPlayer()
  (if (== (Variables|Default|GetIsPlayer) true)
    (Utilities|FlowControl|Sequence
      (:then_0
        ;[1 0.8627 0.2314 1 16] Reset PCoyoteTime
        (if (AI|Components|NavMovement|IsMovingonGround (Variables|Default|GetPlayerMoveCompRef))
          (Variables|Default|SetPHasJumped false)
          (Variables|Default|SetPCoyoteTime (Variables|Default|GetPDefaultCoyoteTime))))
      (:then_1
        ;[1 0.8627 0.2314 1 16] Subtract For CoyoteTime
        (if (Math|Boolean|ANDBoolean (== (Variables|Default|GetPHasJumped) false) (> (Variables|Default|GetPCoyoteTime) 0.0) (not (AI|Components|NavMovement|IsMovingonGround (Variables|Default|GetPlayerMoveCompRef))))
          (Variables|Default|SetPCoyoteTime (- (Variables|Default|GetPCoyoteTime) 1.0)))))))