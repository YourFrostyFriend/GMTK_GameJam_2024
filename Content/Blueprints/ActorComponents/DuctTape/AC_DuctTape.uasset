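; Actor component that lets the player fire duct tape projectiles toward the mouse, limited by ammo held in the game instance.
; On BeginPlay it caches the player, the game instance and the owner's Scalegun component, and enables input on the owner.
; IA_Tape spawns BP_DuctTape_Proj just above the player on a fixed Y plane, rotated toward the Scalegun's mouse location, and spends one tape if item use is allowed.
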(event Input|EnhancedActionEvents|EnhancedInputActionIA_Tape
  (params (ActionValue :type Boolean) (ElapsedSeconds :type Float%20%28double-precision%29) (TriggeredSeconds :type Float%20%28double-precision%29) (InputAction :type Input%20Action%20Object%20Reference :default "/Game/Data/Input/InputActions/IA_Tape.IA_Tape"))
  (bind _gameinstanceref (Variables|Default|GetGameInstanceRef))
  (bind _playerref (Variables|Default|GetPlayerRef))
  (bind _returnvalue (Transformation|GetActorLocation _playerref))
  (:Started
    (if (and (Variables|/Game/Blueprints/Actors/Player/BP_Player.BP_Player_C|GetplyCanUseItems _playerref) (> (Variables|/Game/Blueprints/Utility/Transitions/BP_Game_Instance.BP_Game_Instance_C|GetDuctTapeAmount (Variables|Default|GetGameInstanceRef)) 0))
      (Game|SpawnActorfromClass "/Game/Blueprints/Actors/DuctTape/BP_DuctTape_Proj.BP_DuctTape_Proj_C" (Math|Transform|MakeTransform (Math|Vector|MakeVector (.x _returnvalue) 0.5 (+ (.z _returnvalue) 3e+01)) (Math|Rotator|FindLookatRotation (Math|Vector|MakeVector (.x _returnvalue) (.y _returnvalue) (.z _returnvalue)) (Variables|/Game/Blueprints/ActorComponents/Items/AC_Scalegun.AC_Scalegun_C|GetcurMouseLocation (Variables|Default|GetScalegunComponent))) "1.000000,1.000000,1.000000") "AlwaysSpawn" "MultiplyWithRoot" 0 _playerref)
      (Development|PrintText "TAPED")
      (Variables|/Game/Blueprints/Utility/Transitions/BP_Game_Instance.BP_Game_Instance_C|SetDuctTapeAmount _gameinstanceref (- (Variables|/Game/Blueprints/Utility/Transitions/BP_Game_Instance.BP_Game_Instance_C|GetDuctTapeAmount _gameinstanceref) 1)))))

(event EventBeginPlay
  (Variables|Default|SetScalegunComponent (Actor|GetComponentbyClass (Components|GetOwner) "/Game/Blueprints/ActorComponents/Items/AC_Scalegun.AC_Scalegun_C"))
  (bind _returnvalue (Actor|GetActorOfClass "/Game/Blueprints/Actors/Player/BP_Player.BP_Player_C"))
  (Variables|Default|SetPlayerRef _returnvalue)
  (Input|EnableInput (Components|GetOwner) (Game|GetPlayerController 0))
  (bind _asbp_game_instance (Utilities|Casting|CastToBP_Game_Instance (Game|GetGameInstance)))
  (Variables|Default|SetGameInstanceRef _asbp_game_instance))

(event EventTick
  (params (DeltaSeconds :type Float%20%28single-precision%29)))