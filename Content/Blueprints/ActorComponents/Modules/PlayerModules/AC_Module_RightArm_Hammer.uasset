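; Player module component for a right-arm hammer that performs a two-hit melee swing, triggered by the IA_LeftArm_Click input action.
; A press off cooldown calls PSwingHammer after two successive delays, each spawning a BP_DamageSpace_Box at the owner's current transform with the owner and hammer damage.
; The cooldown is set at swing start and end, and counts down per tick rather than by delta time, pausing mid-swing.
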(event Input|EnhancedActionEvents|EnhancedInputActionIA_LeftArm_Click
  (params (ActionValue :type Boolean) (ElapsedSeconds :type Float%20%28double-precision%29) (TriggeredSeconds :type Float%20%28double-precision%29) (InputAction :type Input%20Action%20Object%20Reference :default "/Game/Data/Input/InputActions/IA_LeftArm_Click.IA_LeftArm_Click"))
  (bind _returnvalue (Components|GetOwner))
  (bind _hammerdamage (Variables|Default|GetHammerDamage))
  (bind _returnvalue_2 (Transformation|GetActorTransform _returnvalue))
  (:Started
    (if (<= (Variables|Default|GetModuleCooldown) 0.0)
      (Utilities|FlowControl|Sequence
        (:then_0
          (Development|PrintString "Hammer Attack!"))
        (:then_1
          (Variables|Default|SetIsSwinging true))
        (:then_2
          (Variables|Default|SetModuleCooldown (Variables|Default|GetDefaultModuleCooldown))
          (Utilities|FlowControl|Delay 0.2)
          (CallFunction|PSwingHammer() _returnvalue (.x (.location _returnvalue_2)) (.z (.location _returnvalue_2)) (.x (.scale _returnvalue_2)) (.z (.scale _returnvalue_2)) _hammerdamage)
          (Utilities|FlowControl|Delay 0.4)
          (CallFunction|PSwingHammer() _returnvalue (.x (.location _returnvalue_2)) (.z (.location _returnvalue_2)) (.x (.scale _returnvalue_2)) (.z (.scale _returnvalue_2)) _hammerdamage)
          (Variables|Default|SetModuleCooldown (Variables|Default|GetDefaultModuleCooldown))
          (Variables|Default|SetIsSwinging false)))
      (else
        (Development|PrintString "Hammer is on cooldown...")))))

(event EventBeginPlay
  (|CallParentFunction))

(event EventTick
  (params (DeltaSeconds :type Float%20%28single-precision%29))
  ;[1 0.9388 0.2746] Tick for Hammer Cooldown
  (if (and (> (Variables|Default|GetModuleCooldown) 0.0) (not (Variables|Default|GetIsSwinging)))
    (Variables|Default|SetModuleCooldown (- (Variables|Default|GetModuleCooldown) 1.0))))

(fn PSwingHammer()
  (params (Source :type Actor%20Object%20Reference) (posX :type Float%20%28double-precision%29) (posZ :type Float%20%28double-precision%29) (scaleX :type Float%20%28double-precision%29) (scaleZ :type Float%20%28double-precision%29) (Amount :type Float%20%28double-precision%29))
  (bind _returnvalue (Components|GetOwner))
  (bind _returnvalue_2 (Transformation|GetActorTransform _returnvalue))
  (Game|SpawnActorfromClass "/Game/Blueprints/Actors/DamageSpace/DamageSpace_Types/DamageSpace_Box/BP_DamageSpace_Box.BP_DamageSpace_Box_C" (Math|Transform|MakeTransform (Math|Vector|MakeVector posX (.y (.location _returnvalue_2)) posZ) (.rotation _returnvalue_2) (Math|Vector|MakeVector scaleX (.y (.scale _returnvalue_2)) scaleZ)) "AlwaysSpawn" "MultiplyWithRoot" 0 (Utilities|Struct|MakeSTRUCT_DamageInfo Source 0 Amount "NewEnumerator0") 0))